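; BP_PowerUpHealth is a one-use health pickup for the ThirdPersonCharacter.
; Its Box trigger starts generating overlap events one second after BeginPlay.
; When the character overlaps it, the pickup adds a fixed amount of Health, clamped to the 0–100 range.
; It then hides the Cube mesh and disables the Box collision rather than destroying the actor.
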(event OnComponentBeginOverlap(Box)
  (params (OverlappedComponent :type Primitive%20Component%20Object%20Reference) (OtherActor :type Actor%20Object%20Reference) (OtherComp :type Primitive%20Component%20Object%20Reference) (OtherBodyIndex :type Integer) (bFromSweep :type Boolean) (SweepResult :type Hit%20Result%20Structure%20%28by%20ref%29))
  (bind _asthird_person_character (Utilities|Casting|CastToThirdPersonCharacter OtherActor))
  (Variables|/Game/ThirdPersonContent/ThirdPersonBP/Blueprints/ThirdPersonCharacter.ThirdPersonCharacter_C|Sethealth _asthird_person_character (Math|Float|Clamp(Float) (+ (Variables|/Game/ThirdPersonContent/ThirdPersonBP/Blueprints/ThirdPersonCharacter.ThirdPersonCharacter_C|Gethealth _asthird_person_character) 34.0) 0.0 1e+02))
  (Rendering|SetVisibility (Variables|Default|GetCube) false false)
  (Components|Activation|SetActive (Variables|Default|GetCube) true false)
  (Collision|SetCollisionEnabled (Variables|Default|GetBox) "NoCollision"))

(event EventBeginPlay
  (Utilities|FlowControl|Delay 1.0)
  (Variables|/Script/Engine.PrimitiveComponent|SetbGenerateOverlapEvents (Variables|Default|GetBox) true))

(event Collision|EventActorBeginOverlap
  (params (OtherActor :type Actor%20Object%20Reference)))

(event EventTick
  (params (DeltaSeconds :type Float%20%28single-precision%29)))

(fn ConstructionScript)