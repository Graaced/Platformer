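; BP_Coins is a coin pickup that adds its Coin value to the player's TotalCoin when collected.
; Its Sphere's begin-overlap event casts the other actor to ThirdPersonCharacter and writes the new total directly on that character.
; The Sphere then hides itself without propagating to children and disables its collision to block repeat pickups; the actor is never destroyed.
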(event OnComponentBeginOverlap(Sphere)
  (params (OverlappedComponent :type Primitive%20Component%20Object%20Reference) (OtherActor :type Actor%20Object%20Reference) (OtherComp :type Primitive%20Component%20Object%20Reference) (OtherBodyIndex :type Integer) (bFromSweep :type Boolean) (SweepResult :type Hit%20Result%20Structure%20%28by%20ref%29))
  (bind _asthird_person_character (Utilities|Casting|CastToThirdPersonCharacter OtherActor))
  (Variables|/Game/ThirdPersonContent/ThirdPersonBP/Blueprints/ThirdPersonCharacter.ThirdPersonCharacter_C|SettotalCoin _asthird_person_character (+ (Variables|/Game/ThirdPersonContent/ThirdPersonBP/Blueprints/ThirdPersonCharacter.ThirdPersonCharacter_C|GettotalCoin _asthird_person_character) (Variables|Default|GetCoin)))
  (Rendering|SetVisibility (Variables|Default|GetSphere) false false)
  (Components|Activation|SetActive (Variables|Default|GetSphere) true false)
  (Collision|SetCollisionEnabled (Variables|Default|GetSphere) "NoCollision"))

(fn ConstructionScript)