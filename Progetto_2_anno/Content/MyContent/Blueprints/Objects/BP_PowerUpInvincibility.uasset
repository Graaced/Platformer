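; BP_PowerUpInvincibility is a pickup that temporarily boosts the health of the overlapping ThirdPersonCharacter.
; A Box overlap hides the Cone, adds 100 Health, then waits ten seconds before setting Health to a flat 100.
; Box collision is disabled only after that delay, and the final step activates the Cone component without restoring its visibility.
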(event OnComponentBeginOverlap(Box)
  (params (OverlappedComponent :type Primitive%20Component%20Object%20Reference) (OtherActor :type Actor%20Object%20Reference) (OtherComp :type Primitive%20Component%20Object%20Reference) (OtherBodyIndex :type Integer) (bFromSweep :type Boolean) (SweepResult :type Hit%20Result%20Structure%20%28by%20ref%29))
  (bind _asthird_person_character (Utilities|Casting|CastToThirdPersonCharacter OtherActor))
  (Rendering|SetVisibility (Variables|Default|GetCone) false false)
  (Variables|/Game/ThirdPersonContent/ThirdPersonBP/Blueprints/ThirdPersonCharacter.ThirdPersonCharacter_C|Sethealth _asthird_person_character (+ (Variables|/Game/ThirdPersonContent/ThirdPersonBP/Blueprints/ThirdPersonCharacter.ThirdPersonCharacter_C|Gethealth _asthird_person_character) 1e+02))
  (Utilities|FlowControl|Delay 1e+01)
  (Variables|/Game/ThirdPersonContent/ThirdPersonBP/Blueprints/ThirdPersonCharacter.ThirdPersonCharacter_C|Sethealth _asthird_person_character 1e+02)
  (Collision|SetCollisionEnabled (Variables|Default|GetBox) "NoCollision")
  (Components|Activation|SetActive (Variables|Default|GetCone) true false))

(fn ConstructionScript)