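; Coin-gated double door that swings open when the ThirdPersonCharacter enters its collision with enough coins.
; On overlap it compares the character's TotalCoin against CoinRequiredAmount, then plays the DoorOpen timeline to drive the relative yaw of both door panels.
; With too few coins it prints a warning whose coin count is hardcoded rather than read from CoinRequiredAmount.
; The graph has no closing logic.
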(event OnComponentBeginOverlap(DoorCollision)
  (params (OverlappedComponent :type Primitive%20Component%20Object%20Reference) (OtherActor :type Actor%20Object%20Reference) (OtherComp :type Primitive%20Component%20Object%20Reference) (OtherBodyIndex :type Integer) (bFromSweep :type Boolean) (SweepResult :type Hit%20Result%20Structure%20%28by%20ref%29))
  (bind _asthird_person_character (Utilities|Casting|CastToThirdPersonCharacter OtherActor))
  (if (>= (Variables|/Game/ThirdPersonContent/ThirdPersonBP/Blueprints/ThirdPersonCharacter.ThirdPersonCharacter_C|GettotalCoin _asthird_person_character) (Variables|Default|GetCoinRequiredAmount))
    (bind (_direction _doorsx _doordx) (Timeline|DoorOpen Play)
      (:Update
        (bind _output_get (Variables|Default|SetDoorSxOpenRotation _doorsx))
        (bind _output_get_2 (Variables|Default|SetDoorDxOpenRotation _doordx))
        (Transformation|SetRelativeRotation (Variables|Default|GetDoorDX) (Math|Rotator|MakeRotator 0.0 0.0 (.z _output_get_2)) false false)
        (Transformation|SetRelativeRotation (Variables|Default|GetDoorSX) (Math|Rotator|MakeRotator 0.0 0.0 (.z _output_get)) false false)))
    (else
      (Development|PrintString "You Need 6 Coins Total !" true true "(R=1.000000,G=0.074021,B=0.000000,A=1.000000)"))))

(fn ConstructionScript)