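; BP_PowerUpBox is a bump box that releases a random pickup when a ThirdPersonCharacter overlaps its Box.
; Each overlap raises the root with MoveComponentTo, then reaches a DoOnce that gates everything after.
; The first pass randomly spawns coins, a health power-up or an invincibility power-up at the Arrow's transform, then lowers the box after a short delay.
; Later overlaps only raise it, with no drop or return.
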(event OnComponentBeginOverlap(Box)
  (params (OverlappedComponent :type Primitive%20Component%20Object%20Reference) (OtherActor :type Actor%20Object%20Reference) (OtherComp :type Primitive%20Component%20Object%20Reference) (OtherBodyIndex :type Integer) (bFromSweep :type Boolean) (SweepResult :type Hit%20Result%20Structure%20%28by%20ref%29))
  (bind _defaultsceneroot (Variables|Default|GetDefaultSceneRoot))
  (bind _defaultsceneroot_2 (Variables|Default|GetDefaultSceneRoot))
  (bind _returnvalue (Transformation|GetRelativeTransform _defaultsceneroot_2))
  (Utilities|Casting|CastToThirdPersonCharacter OtherActor)
  (Components|MoveComponentTo _defaultsceneroot_2 (+ (.location _returnvalue) "0, 0,60.000000") (.rotation _returnvalue) false false 0.1 false)
  (Utilities|FlowControl|DoOnce false
    (:Completed
      (switch int (Math|Random|RandomIntegerinRange 0 2)
        (:0
          (CallFunction|SpawnCoins))
        (:1
          (CallFunction|SpawnPwHealth))
        (:2
          (CallFunction|SpawnPwInv)))
      (Utilities|FlowControl|Delay 0.3)
      (Components|MoveComponentTo _defaultsceneroot (+ (.location (Transformation|GetRelativeTransform _defaultsceneroot)) "0, 0,-60.000000") "0, 0, 0" false false 0.1 false)
      (Utilities|FlowControl|Delay 0.5))))

(event Custom|SpawnPwInv
  (Game|SpawnActorfromClass "/Game/MyContent/Blueprints/Objects/BP_PowerUpInvincibility.BP_PowerUpInvincibility_C" (Transformation|GetWorldTransform (Variables|Default|GetArrow)) "Undefined" 0 0))

(event Custom|SpawnCoins
  (Game|SpawnActorfromClass "/Game/MyContent/Blueprints/Objects/BP_Coins.BP_Coins_C" (Transformation|GetWorldTransform (Variables|Default|GetArrow)) "Undefined" 0 0))

(event Custom|SpawnPwHealth
  (Game|SpawnActorfromClass "/Game/MyContent/Blueprints/Objects/BP_PowerUpHealth.BP_PowerUpHealth_C" (Transformation|GetWorldTransform (Variables|Default|GetArrow)) "Undefined" 0 0))

(fn ConstructionScript)