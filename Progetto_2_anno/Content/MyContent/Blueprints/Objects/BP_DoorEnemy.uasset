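; BP_DoorEnemy is a double door that stays shut until the player has reached a required enemy count.
; When a ThirdPersonCharacter overlaps DoorCollision, it compares the character's TotalEnemy to EnemyRequiredAmount and prints a red warning to kill all enemies if it falls short.
; Otherwise OpenDoor plays a timeline that drives the yaw of the left and right door leaves to swing them open.
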(event OnComponentBeginOverlap(DoorCollision)
  (params (OverlappedComponent :type Primitive%20Component%20Object%20Reference) (OtherActor :type Actor%20Object%20Reference) (OtherComp :type Primitive%20Component%20Object%20Reference) (OtherBodyIndex :type Integer) (bFromSweep :type Boolean) (SweepResult :type Hit%20Result%20Structure%20%28by%20ref%29))
  (bind _asthird_person_character (Utilities|Casting|CastToThirdPersonCharacter OtherActor))
  (if (>= (Variables|/Game/ThirdPersonContent/ThirdPersonBP/Blueprints/ThirdPersonCharacter.ThirdPersonCharacter_C|GettotalEnemy _asthird_person_character) (Variables|Default|GetEnemy%20Required%20Amount))
    (CallFunction|OpenDoor)
    (else
      (Development|PrintString "You must kill all the enemies first to be able to continue " true true "(R=1.000000,G=0.105803,B=0.225562,A=1.000000)"))))

(event Custom|OpenDoor
  (bind (_direction _doorsx _doordx) (Timeline|OpenDoorTimeLine Play)
    (:Update
      (bind _output_get (Variables|Default|SetDoorSxOpenRotation _doorsx))
      (bind _output_get_2 (Variables|Default|SetDoorDxOpenRotation _doordx))
      (Transformation|SetRelativeRotation (Variables|Default|GetDoorDX) (Math|Rotator|MakeRotator 0.0 0.0 (.z _output_get_2)) false false)
      (Transformation|SetRelativeRotation (Variables|Default|GetDoorSX) (Math|Rotator|MakeRotator 0.0 0.0 (.z _output_get)) false false))))

(fn ConstructionScript)