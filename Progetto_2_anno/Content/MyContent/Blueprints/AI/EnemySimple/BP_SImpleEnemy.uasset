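; BP_SImpleEnemy is a simple enemy that is defeated when a ThirdPersonCharacter overlaps its head collision box.
; The overlap calls DropLoot, adds EnemySimple to the character's TotalEnemy count, then destroys the enemy.
; DropLoot traces down to place a random pickup at the hit location.
; Its RandomInteger(2) selection only yields coins or health, leaving the invincibility option unreachable.
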(event OnComponentBeginOverlap(HeadBoxCollision)
  (params (OverlappedComponent :type Primitive%20Component%20Object%20Reference) (OtherActor :type Actor%20Object%20Reference) (OtherComp :type Primitive%20Component%20Object%20Reference) (OtherBodyIndex :type Integer) (bFromSweep :type Boolean) (SweepResult :type Hit%20Result%20Structure%20%28by%20ref%29))
  (bind _asthird_person_character (Utilities|Casting|CastToThirdPersonCharacter OtherActor))
  (CallFunction|DropLoot)
  (Variables|/Game/ThirdPersonContent/ThirdPersonBP/Blueprints/ThirdPersonCharacter.ThirdPersonCharacter_C|SettotalEnemy _asthird_person_character (+ (Variables|/Game/ThirdPersonContent/ThirdPersonBP/Blueprints/ThirdPersonCharacter.ThirdPersonCharacter_C|GettotalEnemy _asthird_person_character) (Variables|Default|GetEnemySimple)))
  (Actor|DestroyActor))

(event Custom|DropLoot
  (bind _returnvalue (Transformation|GetActorLocation))
  ;[1 1 1] RandomLootSpawn
  (bind _outhit (Collision|LineTraceByChannel _returnvalue (- _returnvalue "0, 0,500.000000") "TraceTypeQuery1" false (Utilities|Array|MakeArray (Game|GetPlayerCharacter 0)) "None"))
  (Game|SpawnActorfromClass (Utilities|Select :Index (Math|Random|RandomInteger 2) :Option%200 "/Game/MyContent/Blueprints/Objects/BP_Coins.BP_Coins_C" :Option%201 "/Game/MyContent/Blueprints/Objects/BP_PowerUpHealth.BP_PowerUpHealth_C" :Option%202 "/Game/MyContent/Blueprints/Objects/BP_PowerUpInvincibility.BP_PowerUpInvincibility_C") (Math|Transform|MakeTransform (.Location (Collision|BreakHitResult _outhit))) "Undefined" 0 0))

(fn ConstructionScript)